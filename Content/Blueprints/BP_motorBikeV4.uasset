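; Motorbike actor that moves along a BP_MotorPathSpline and animates its steering.
; BeginPlay caches the anim instance, takes the spline at index 2 and calls Move, which restarts a timeline inside a per-segment loop, flagged as faulty.
; An alternative point-by-point myMove, also flagged, is not called from BeginPlay.
; Tick sends speed and an interpolated steering angle, chosen by the sign of world yaw, to the AnimBlueprint.
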(event Custom|Move
  (bind _spline_ref (Variables|Default|GetSpline%20REF))
  (bind _spline_ref_2 (Variables|Default|GetSpline%20REF))
  (bind _spline_ref_3 (Variables|Default|GetSpline%20REF))
  (bind _spline (Variables|/Game/Blueprints/BP_MotorPathSpline.BP_MotorPathSpline_C|GetSpline _spline_ref_2))
  (bind _spline_2 (Variables|/Game/Blueprints/BP_MotorPathSpline.BP_MotorPathSpline_C|GetSpline _spline_ref))
  (bind _spline_3 (Variables|/Game/Blueprints/BP_MotorPathSpline.BP_MotorPathSpline_C|GetSpline _spline_ref_3))
  (bind _returnvalue (Spline|GetNumberOfSplinePoints _spline))
  ;[1 1 1] Non funziona bene con il for
  (Variables|Default|SetTime%20to%20Complete%28sec%29 (* _returnvalue 0.02))
  (for _index (range 0 (- _returnvalue 2))
    (Components|Timeline|SetPlayRate (Variables|Default|GetMoveObject) 1.0)
    (bind _moveobject (Timeline|Timeline PlayFromStart)
      (:Update
        (Transformation|SetActorTransform (Math|Transform|MakeTransform (Spline|GetLocationatDistanceAlongSpline _spline_3 (Math|Float|Lerp (Spline|GetDistanceAlongSplineatSplinePoint _spline_2 (+ _index 1)) (Spline|GetDistanceAlongSplineatSplinePoint _spline_2 _index) _moveobject) "World") (Math|Rotator|MakeRotator 0.0 0.0 (.yaw (Spline|GetRotationatDistanceAlongSpline _spline_3 (Math|Float|Lerp (Spline|GetDistanceAlongSplineatSplinePoint _spline_2 (+ _index 1)) (Spline|GetDistanceAlongSplineatSplinePoint _spline_2 _index) _moveobject) "Local"))) "1.000000,1.000000,1.000000"))
        (Variables|Default|SetInclinazione%20corrente (Math|Interpolation|FInterpTo (Variables|Default|GetInclinazione%20corrente) (Variables|Default|GetAngolo%20di%20sterzata%20corremte) (Utilities|Time|GetWorldDeltaSeconds) 0.5))))))

(event Custom|myMove
  (bind _spline_ref (Variables|Default|GetSpline%20REF))
  (bind _spline_ref_2 (Variables|Default|GetSpline%20REF))
  (bind _spline (Variables|/Game/Blueprints/BP_MotorPathSpline.BP_MotorPathSpline_C|GetSpline _spline_ref))
  (bind _spline_2 (Variables|/Game/Blueprints/BP_MotorPathSpline.BP_MotorPathSpline_C|GetSpline _spline_ref_2))
  ;[1 1 1] Non funziona come dovrebbe su percorsi più lunghi e fitti di punti.
  (Variables|Default|SetLastIndexOfSpline (- (Spline|GetNumberOfSplinePoints (Variables|/Game/Blueprints/BP_MotorPathSpline.BP_MotorPathSpline_C|GetSpline (Variables|Default|GetSpline%20REF))) 1))
  (Components|Timeline|SetPlayRate (Variables|Default|GetMoveObject) 5e+01)
  (bind _moveobject (Timeline|MoveObject PlayFromStart)
    (:Update
      (Transformation|SetActorTransform (Math|Transform|MakeTransform (Spline|GetLocationatDistanceAlongSpline _spline_2 (Math|Float|Lerp (Spline|GetDistanceAlongSplineatSplinePoint _spline (Variables|Default|GetCurrentSplinePoint)) (Spline|GetDistanceAlongSplineatSplinePoint _spline (+ (Variables|Default|GetCurrentSplinePoint) 1)) _moveobject) "World") (Math|Rotator|MakeRotator 0.0 0.0 (.yaw (Spline|GetRotationatDistanceAlongSpline _spline_2 (Math|Float|Lerp (Spline|GetDistanceAlongSplineatSplinePoint _spline (Variables|Default|GetCurrentSplinePoint)) (Spline|GetDistanceAlongSplineatSplinePoint _spline (+ (Variables|Default|GetCurrentSplinePoint) 1)) _moveobject) "Local"))) "1.000000,1.000000,1.000000"))
      (if (Utilities|Operators|EqualEqual (Transformation|GetActorLocation) (Spline|GetLocationatSplinePoint (Variables|/Game/Blueprints/BP_MotorPathSpline.BP_MotorPathSpline_C|GetSpline (Variables|Default|GetSpline%20REF)) (+ (Variables|Default|GetCurrentSplinePoint) 1) "World") 0.0)
        (Variables|Default|SetCurrentSplinePoint (+ (Variables|Default|GetCurrentSplinePoint) 1))))
    (:Finished
      (if (!= (Variables|Default|GetCurrentSplinePoint) (Variables|Default|GetLastIndexOfSpline))
        (CallFunction|MyMove)
        (else
          (Development|PrintString "Percorso terminato"))))))

(event EventBeginPlay
  (bind _asfuturistic_motorbike_skeleton_anim_blueprint (Utilities|Casting|CastTofuturistic_motorbike_Skeleton_AnimBlueprint (Components|SkeletalMesh|GetAnimInstance (Variables|Default|GetMotorBike))))
  (Variables|Default|SetAnimInstance _asfuturistic_motorbike_skeleton_anim_blueprint)
  (bind _outactors (Actor|GetAllActorsOfClass "/Game/Blueprints/BP_MotorPathSpline.BP_MotorPathSpline_C"))
  (Variables|Default|SetSpline%20REF (Utilities|Array|Get(acopy) _outactors 2))
  (CallFunction|Move))

(fn ConstructionScript)

(event EventTick
  (params (DeltaSeconds :type Float%20%28single-precision%29))
  (bind _returnvalue (Transformation|GetActorRotation))
  (Variables|/Game/Blueprints/futuristic_motorbike_Skeleton_AnimBlueprint.futuristic_motorbike_Skeleton_AnimBlueprint_C|Setvelocità%20moto (Variables|Default|GetAnimInstance) (Variables|Default|GetcurrentSpeed))
  (if (> (.yaw _returnvalue) 0.0)
    (bind _output_get (Variables|Default|SetAngolo%20di%20sterzata%20corremte (Math|Interpolation|FInterpTo (Variables|Default|GetAngolo%20di%20sterzata%20corremte) (Variables|Default|GetMassimo%20angolo%20di%20sterzata) (Utilities|Time|GetWorldDeltaSeconds) 2.0)))
    (Variables|/Game/Blueprints/futuristic_motorbike_Skeleton_AnimBlueprint.futuristic_motorbike_Skeleton_AnimBlueprint_C|SetAngolo%20di%20sterzata (Variables|Default|GetAnimInstance) _output_get)
    (elif (< (.yaw _returnvalue) 0.0)
      (bind _output_get_2 (Variables|Default|SetAngolo%20di%20sterzata%20corremte (Math|Interpolation|FInterpTo (Variables|Default|GetAngolo%20di%20sterzata%20corremte) (* (Variables|Default|GetMassimo%20angolo%20di%20sterzata) -1.0) (Utilities|Time|GetWorldDeltaSeconds) 2.0)))
      (Variables|/Game/Blueprints/futuristic_motorbike_Skeleton_AnimBlueprint.futuristic_motorbike_Skeleton_AnimBlueprint_C|SetAngolo%20di%20sterzata (Variables|Default|GetAnimInstance) _output_get_2)
      (else
        (Variables|/Game/Blueprints/futuristic_motorbike_Skeleton_AnimBlueprint.futuristic_motorbike_Skeleton_AnimBlueprint_C|SetAngolo%20di%20sterzata (Variables|Default|GetAnimInstance) 0.0)))))