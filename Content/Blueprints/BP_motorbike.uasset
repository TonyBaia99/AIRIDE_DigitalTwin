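; Player-driven motorbike Blueprint that handles movement, steering, lean and a spring-arm look camera.
; Throttle and steering axes ease speed and steer angle toward their targets with FInterpTo.
; Tick moves the actor forward with a swept offset, yaws it by speed times steer angle (doubled in reverse) and interpolates roll to lean with speed.
; It also feeds speed and steer angle, damped at higher speed, to the bike's animation Blueprint.
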(event EventBeginPlay
  ;[1 1 1] Questa parte è necessaria per recuperare il riferimento al Blueprint dove verrano generate le animazioni
  (bind _asfuturistic_motorbike_skeleton_anim_blueprint (Utilities|Casting|CastTofuturistic_motorbike_Skeleton_AnimBlueprint (Components|SkeletalMesh|GetAnimInstance (Variables|Default|GetMotorBike))))
  (Variables|Default|SetAnimInstance _asfuturistic_motorbike_skeleton_anim_blueprint))

(event EventTick
  (params (DeltaSeconds :type Float%20%28single-precision%29))
  (bind _animinstance (Variables|Default|GetAnimInstance))
  (bind _current_speed (Variables|Default|GetCurrent%20speed))
  ;[1 1 1 1 16] Porzione di codice necessaria a far muovere la moto avanti o indietro, cioè alla posizione corrente nelle moto in coordinate globali viene aggiunto un delta che dipende dalla velocità corrente.
  (Transformation|AddActorWorldOffset (* DeltaSeconds (* (Transformation|GetActorForwardVector) _current_speed)) true)
  (Transformation|SetActorRelativeRotation (Math|Rotator|MakeRotator (Math|Interpolation|FInterpTo (Variables|Default|GetInclinazione%20corrente) (* (Variables|Default|GetAngolo%20di%20sterzata%20corrente) (/ (Variables|Default|GetCurrent%20speed) (Variables|Default|GetMaxSpeed))) (Utilities|Time|GetWorldDeltaSeconds) 5.0) 0.0 (+ (.yaw (Transformation|GetActorRotation)) (* _current_speed (Variables|Default|GetAngolo%20di%20sterzata%20corrente) (Variables|Default|GetSpeedToRotation%20Factor) (Utilities|Time|GetWorldDeltaSeconds) (select (< _current_speed 0.0) 2.0 1.0)))))
  (Variables|Default|SetInclinazione%20corrente (Math|Interpolation|FInterpTo (Variables|Default|GetInclinazione%20corrente) (* (Variables|Default|GetAngolo%20di%20sterzata%20corrente) (/ (Variables|Default|GetCurrent%20speed) (Variables|Default|GetMaxSpeed))) (Utilities|Time|GetWorldDeltaSeconds) 5.0))
  ;[1 1 1] Con questo pezzo stiamo impostato i valori di velocità e sterzata così che abbiano effetto sul blueprint di animazione della moto
  (Variables|/Game/Blueprints/futuristic_motorbike_Skeleton_AnimBlueprint.futuristic_motorbike_Skeleton_AnimBlueprint_C|Setvelocità%20moto _animinstance (Variables|Default|GetCurrent%20speed))
  (Variables|/Game/Blueprints/futuristic_motorbike_Skeleton_AnimBlueprint.futuristic_motorbike_Skeleton_AnimBlueprint_C|SetAngolo%20di%20sterzata _animinstance (* (Variables|Default|GetAngolo%20di%20sterzata%20corrente) (Math|Float|MapRangeClamped (Variables|Default|GetCurrent%20speed) 0.0 (Variables|Default|GetMaxSpeed) 1.0 0.2))))

(event Input|AxisEvents|InputAxisAccelleratore
  (params (AxisValue :type Float%20%28single-precision%29))
  ;[0 0.227 1 1 14] Questa parte è necessaria per gestire l'accellerazione della moto. Fatto in modo tale che la moto accelleri e decelleri il più realisticamenete possibile utilizzando un nodo di interpolazione.
  (Variables|Default|SetCurrent%20speed (Math|Interpolation|FInterpTo (Variables|Default|GetCurrent%20speed) (* AxisValue (Variables|Default|GetMaxSpeed)) (Utilities|Time|GetWorldDeltaSeconds) 4.0)))

(event Input|AxisEvents|InputAxisSterzo
  (params (AxisValue :type Float%20%28single-precision%29))
  ;[0 0 1] Questa parte gestisce la moto che gira, e cioè la sterzata, rendendola il più realisitca possibile facendo in modo tale che la sterzata avvenga gradualmente
  (Variables|Default|SetAngolo%20di%20sterzata%20corrente (Math|Interpolation|FInterpTo (Variables|Default|GetAngolo%20di%20sterzata%20corrente) (* AxisValue (Variables|Default|GetMassimo%20angolo%20di%20sterzo)) (Utilities|Time|GetWorldDeltaSeconds) 4.0)))

(event Input|AxisEvents|InputAxisLook_up
  (params (AxisValue :type Float%20%28single-precision%29))
  ;[0 0 1 1 14] Parte necessaria per spostare la telecamera che segue la moto
  (Transformation|AddRelativeRotation (Variables|Default|GetSpringArm) (Math|Rotator|MakeRotator 0.0 AxisValue 0.0) false false))

(event Input|AxisEvents|InputAxisLook_right
  (params (AxisValue :type Float%20%28single-precision%29))
  ;[0 0 1 1 14] Parte necessaria per spostare la telecamera che segue la moto
  (Transformation|AddRelativeRotation (Variables|Default|GetSpringArm) (Math|Rotator|MakeRotator 0.0 0.0 AxisValue) false false))

(fn ConstructionScript)