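; Motorbike actor that rides a BP_MotorPathSpline, picked by SplineIndex, and pauses the game at the last point.
; BeginPlay precomputes per-segment speed and acceleration assuming 0.02 s between points, then starts Move.
; Move runs a fast timeline per segment, setting location and yaw, which the author notes is machine-dependent and unreliable on long, dense paths.
; Tick is empty; anim steering/velocity, debug arrow and MoveV2 logic are disconnected.
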(event Custom|calculateSpeed
  (bind _spline_ref (Variables|Default|GetSpline%20REF))
  (bind _spline (Variables|/Game/Blueprints/BP_MotorPathSpline.BP_MotorPathSpline_C|GetSpline _spline_ref))
  ;[1 1 1] Metodo che calcola le velocità che la   moto fa percorrendo la spline
  (for _index (range 0 (- (Spline|GetNumberOfSplinePoints (Variables|/Game/Blueprints/BP_MotorPathSpline.BP_MotorPathSpline_C|GetSpline (Variables|Default|GetSpline%20REF))) 2))
    (Utilities|Array|Add (Variables|Default|GetspeedAlongSpline) (/ (/ (- (Spline|GetDistanceAlongSplineatSplinePoint _spline (+ _index 1)) (Spline|GetDistanceAlongSplineatSplinePoint _spline _index)) 0.02) 1e+04))))

(event Custom|Move
  (bind _spline_ref (Variables|Default|GetSpline%20REF))
  (bind _spline (Variables|/Game/Blueprints/BP_MotorPathSpline.BP_MotorPathSpline_C|GetSpline _spline_ref))
  ;[1 1 1] Non funziona come dovrebbe su percorsi più lunghi e fitti di punti. Dipende troppo dalla potenza della macchina
  (Variables|Default|SetLastIndexOfSpline (- (Spline|GetNumberOfSplinePoints (Variables|/Game/Blueprints/BP_MotorPathSpline.BP_MotorPathSpline_C|GetSpline (Variables|Default|GetSpline%20REF))) 1))
  (Components|Timeline|SetPlayRate (Variables|Default|GetMoveObject) 5e+01)
  (bind _moveobject (Timeline|MoveObject PlayFromStart)
    (:Update
      (Transformation|SetActorTransform (Math|Transform|MakeTransform (.location (Spline|GetTransformatDistanceAlongSpline _spline (Math|Float|Lerp (Spline|GetDistanceAlongSplineatSplinePoint _spline (Variables|Default|GetCurrentSplinePoint)) (Spline|GetDistanceAlongSplineatSplinePoint _spline (+ (Variables|Default|GetCurrentSplinePoint) 1)) _moveobject) "World" false)) (Math|Rotator|MakeRotator 0.0 0.0 (* (.yaw (.rotation (Spline|GetTransformatDistanceAlongSpline _spline (Math|Float|Lerp (Spline|GetDistanceAlongSplineatSplinePoint _spline (Variables|Default|GetCurrentSplinePoint)) (Spline|GetDistanceAlongSplineatSplinePoint _spline (+ (Variables|Default|GetCurrentSplinePoint) 1)) _moveobject) "World" false))) 1.0)) "1.000000,1.000000,1.000000"))
      (if (Utilities|Operators|EqualEqual (Transformation|GetActorLocation) (Spline|GetLocationatSplinePoint (Variables|/Game/Blueprints/BP_MotorPathSpline.BP_MotorPathSpline_C|GetSpline (Variables|Default|GetSpline%20REF)) (+ (Variables|Default|GetCurrentSplinePoint) 1) "World") 0.0)
        (Variables|Default|SetCurrentSplinePoint (+ (Variables|Default|GetCurrentSplinePoint) 1))))
    (:Finished
      (if (!= (Variables|Default|GetCurrentSplinePoint) (Variables|Default|GetLastIndexOfSpline))
        (Timeline|MoveObject Play)
        (else
          (Game|SetGamePaused true))))))

(event Custom|calculateAcc
  (bind _speedalongspline (Variables|Default|GetspeedAlongSpline))
  ;[1 1 1] Metodo che calcola le accelerazioni della moto lungo la spline che percorre
  (for _index (range 0 (- (Utilities|Array|Length (Variables|Default|GetspeedAlongSpline)) 2))
    (Utilities|Array|Add (Variables|Default|GetaccAlongSpline) (/ (- (Utilities|Array|Get(acopy) _speedalongspline (+ _index 1)) (Utilities|Array|Get(acopy) _speedalongspline _index)) 0.02))))

(event EventBeginPlay
  (bind _asfuturistic_motorbike_skeleton_anim_blueprint (Utilities|Casting|CastTofuturistic_motorbike_Skeleton_AnimBlueprint (Components|SkeletalMesh|GetAnimInstance (Variables|Default|GetMotorBike))))
  (Variables|Default|SetAnimInstance _asfuturistic_motorbike_skeleton_anim_blueprint)
  (bind _outactors (Actor|GetAllActorsOfClass "/Game/Blueprints/BP_MotorPathSpline.BP_MotorPathSpline_C"))
  (Variables|Default|SetSpline%20REF (Utilities|Array|Get(acopy) _outactors (Variables|Default|GetSplineIndex)))
  (CallFunction|CalculateSpeed)
  (CallFunction|CalculateAcc)
  (CallFunction|Move))

(event EventTick
  (params (DeltaSeconds :type Float%20%28single-precision%29))
  ;[1 1 1] Non funziona come dovrebbe su percorsi più lunghi e fitti di punti. Dipende troppo dalla potenza della macchina
)

(fn ConstructionScript)