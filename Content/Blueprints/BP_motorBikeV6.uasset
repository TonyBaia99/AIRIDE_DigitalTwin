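; Motorbike Blueprint, version 6, that moves the bike along a BP_MotorPathSpline and drives its steering animation.
; On BeginPlay it takes the third path actor found and steps through it with a DoN and Delay loop, setting location and yaw at constant-velocity spline times.
; The author notes this movement, like V5, depends on frame rate.
; Tick feeds speed and an interpolated steering angle, signed by actor yaw, to the AnimBlueprint.
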(event Custom|MoveV2
  (bind _spline_ref (Variables|Default|GetSpline%20REF))
  (bind _spline (Variables|/Game/Blueprints/BP_MotorPathSpline.BP_MotorPathSpline_C|GetSpline _spline_ref))
  ;[1 1 1] Molto simile a V5 ma ha lo stesso problema, dipende molto da quanti fps riesce a fare la macchina
  (bind _output_get (Variables|Default|SetLastIndexOfSpline (- (Spline|GetNumberOfSplinePoints _spline) 1)))
  (bind _output_get_2 (Variables|/Script/Engine.SplineComponent|SetDuration _spline (* _output_get 0.02)))
  (Development|PrintString (Utilities|String|ToString(Float) _output_get_2) true true "(R=1.000000,G=0.000000,B=0.039894,A=1.000000)" 5.0)
  (bind _counter (Utilities|FlowControl|DoN (+ (Variables|Default|GetLastIndexOfSpline) 1) :!label _label)
    (:Exit
      (Development|PrintText (Utilities|Text|ToText(Integer) (- _counter 1)) true true "(R=0.000000,G=0.660000,B=1.000000,A=1.000000)" 0.1)
      (Transformation|SetActorTransform (Math|Transform|MakeTransform (Spline|GetLocationatTime _spline (* (- _counter 1) (/ (Variables|/Script/Engine.SplineComponent|GetDuration (Variables|/Game/Blueprints/BP_MotorPathSpline.BP_MotorPathSpline_C|GetSpline (Variables|Default|GetSpline%20REF))) (Math|Conversions|ToFloat(Integer) (Variables|Default|GetLastIndexOfSpline)))) "World" true) (Math|Rotator|MakeRotator 0.0 0.0 (.yaw (Class|SplineComponent|GetRotationatTime _spline (* (- _counter 1) (/ (Variables|/Script/Engine.SplineComponent|GetDuration (Variables|/Game/Blueprints/BP_MotorPathSpline.BP_MotorPathSpline_C|GetSpline (Variables|Default|GetSpline%20REF))) (Math|Conversions|ToFloat(Integer) (Variables|Default|GetLastIndexOfSpline)))) "Local" true))) "1.000000,1.000000,1.000000"))
      (Utilities|FlowControl|Delay 0.02)
      (goto _label))))

(event EventBeginPlay
  (bind _asfuturistic_motorbike_skeleton_anim_blueprint (Utilities|Casting|CastTofuturistic_motorbike_Skeleton_AnimBlueprint (Components|SkeletalMesh|GetAnimInstance (Variables|Default|GetMotorBike))))
  (Variables|Default|SetAnimInstance _asfuturistic_motorbike_skeleton_anim_blueprint)
  (bind _outactors (Actor|GetAllActorsOfClass "/Game/Blueprints/BP_MotorPathSpline.BP_MotorPathSpline_C"))
  (Variables|Default|SetSpline%20REF (Utilities|Array|Get(acopy) _outactors 2))
  (CallFunction|MoveV2))

(fn ConstructionScript)

(event EventTick
  (params (DeltaSeconds :type Float%20%28single-precision%29))
  (bind _returnvalue (Transformation|GetActorRotation))
  (Variables|/Game/Blueprints/futuristic_motorbike_Skeleton_AnimBlueprint.futuristic_motorbike_Skeleton_AnimBlueprint_C|Setvelocità%20moto (Variables|Default|GetAnimInstance) (Variables|Default|GetcurrentSpeed))
  (if (> (.yaw _returnvalue) 0.0)
    (bind _output_get (Variables|Default|SetAngolo%20di%20sterzata%20corremte (Math|Interpolation|FInterpTo (Variables|Default|GetAngolo%20di%20sterzata%20corremte) (Variables|Default|GetMassimo%20angolo%20di%20sterzata) (Utilities|Time|GetWorldDeltaSeconds) 2.0)))
    (Variables|/Game/Blueprints/futuristic_motorbike_Skeleton_AnimBlueprint.futuristic_motorbike_Skeleton_AnimBlueprint_C|SetAngolo%20di%20sterzata (Variables|Default|GetAnimInstance) _output_get)
    (elif (< (.yaw _returnvalue) 0.0)
      (bind _output_get_2 (Variables|Default|SetAngolo%20di%20sterzata%20corremte (Math|Interpolation|FInterpTo (Variables|Default|GetAngolo%20di%20sterzata%20corremte) (* (Variables|Default|GetMassimo%20angolo%20di%20sterzata) -1.0) (Utilities|Time|GetWorldDeltaSeconds) 2.0)))
      (Variables|/Game/Blueprints/futuristic_motorbike_Skeleton_AnimBlueprint.futuristic_motorbike_Skeleton_AnimBlueprint_C|SetAngolo%20di%20sterzata (Variables|Default|GetAnimInstance) _output_get_2)
      (else
        (Variables|/Game/Blueprints/futuristic_motorbike_Skeleton_AnimBlueprint.futuristic_motorbike_Skeleton_AnimBlueprint_C|SetAngolo%20di%20sterzata (Variables|Default|GetAnimInstance) 0.0)))))