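; Motorbike actor that rides along the first BP_MotorPathSpline found in the level, starting on BeginPlay.
; A timeline scaled by TimeToCompleteSec moves it by spline distance, taking yaw from the spline and easing roll toward the steering angle.
; Tick eases that angle toward plus or minus its maximum by the sign of world yaw, not turn rate.
; It passes steering and CurrentSpeed, never set here, to the animation Blueprint.
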(event Custom|Move
  (bind _spline_ref (Variables|Default|GetSpline%20REF))
  (bind _spline (Variables|/Game/Blueprints/BP_MotorPathSpline.BP_MotorPathSpline_C|GetSpline _spline_ref))
  (Components|Timeline|SetPlayRate (Variables|Default|GetMove%20object) (/ 1.0 (Variables|Default|GetTime%20to%20Complete%28sec%29)))
  (bind _move_track (Timeline|Move%20object PlayFromStart)
    (:Update
      (Transformation|SetActorTransform (Math|Transform|MakeTransform (Spline|GetLocationatDistanceAlongSpline _spline (Math|Float|Lerp 0.0 (Spline|GetSplineLength (Variables|/Game/Blueprints/BP_MotorPathSpline.BP_MotorPathSpline_C|GetSpline (Variables|Default|GetSpline%20REF))) _move_track) "World") (Math|Rotator|MakeRotator (Math|Interpolation|FInterpTo (Variables|Default|GetInclinazione%20corrente) (Variables|Default|GetAngolo%20di%20sterzata%20corremte) (Utilities|Time|GetWorldDeltaSeconds) 0.5) 0.0 (.yaw (Spline|GetRotationatDistanceAlongSpline _spline (Math|Float|Lerp 0.0 (Spline|GetSplineLength (Variables|/Game/Blueprints/BP_MotorPathSpline.BP_MotorPathSpline_C|GetSpline (Variables|Default|GetSpline%20REF))) _move_track) "Local"))) "1.000000,1.000000,1.000000"))
      (Variables|Default|SetInclinazione%20corrente (Math|Interpolation|FInterpTo (Variables|Default|GetInclinazione%20corrente) (Variables|Default|GetAngolo%20di%20sterzata%20corremte) (Utilities|Time|GetWorldDeltaSeconds) 0.5)))))

(event EventBeginPlay
  (bind _asfuturistic_motorbike_skeleton_anim_blueprint (Utilities|Casting|CastTofuturistic_motorbike_Skeleton_AnimBlueprint (Components|SkeletalMesh|GetAnimInstance (Variables|Default|GetMotorBike))))
  (Variables|Default|SetAnimInstance _asfuturistic_motorbike_skeleton_anim_blueprint)
  (bind _returnvalue (Actor|GetActorOfClass "/Game/Blueprints/BP_MotorPathSpline.BP_MotorPathSpline_C"))
  (Variables|Default|SetSpline%20REF _returnvalue)
  (CallFunction|Move))

(event Collision|EventActorBeginOverlap
  (params (OtherActor :type Actor%20Object%20Reference)))

(event EventTick
  (params (DeltaSeconds :type Float%20%28single-precision%29))
  (bind _returnvalue (Transformation|GetActorRotation))
  (Variables|/Game/Blueprints/futuristic_motorbike_Skeleton_AnimBlueprint.futuristic_motorbike_Skeleton_AnimBlueprint_C|Setvelocità%20moto (Variables|Default|GetAnimInstance) (Variables|Default|GetcurrentSpeed))
  (if (> (.yaw _returnvalue) 0.0)
    (bind _output_get (Variables|Default|SetAngolo%20di%20sterzata%20corremte (Math|Interpolation|FInterpTo (Variables|Default|GetAngolo%20di%20sterzata%20corremte) (Variables|Default|GetMassimo%20angolo%20di%20sterzata) (Utilities|Time|GetWorldDeltaSeconds) 2.0)))
    (Variables|/Game/Blueprints/futuristic_motorbike_Skeleton_AnimBlueprint.futuristic_motorbike_Skeleton_AnimBlueprint_C|SetAngolo%20di%20sterzata (Variables|Default|GetAnimInstance) _output_get)
    (elif (< (.yaw _returnvalue) 0.0)
      (bind _output_get_2 (Variables|Default|SetAngolo%20di%20sterzata%20corremte (Math|Interpolation|FInterpTo (Variables|Default|GetAngolo%20di%20sterzata%20corremte) (* (Variables|Default|GetMassimo%20angolo%20di%20sterzata) -1.0) (Utilities|Time|GetWorldDeltaSeconds) 2.0)))
      (Variables|/Game/Blueprints/futuristic_motorbike_Skeleton_AnimBlueprint.futuristic_motorbike_Skeleton_AnimBlueprint_C|SetAngolo%20di%20sterzata (Variables|Default|GetAnimInstance) _output_get_2)
      (else
        (Variables|/Game/Blueprints/futuristic_motorbike_Skeleton_AnimBlueprint.futuristic_motorbike_Skeleton_AnimBlueprint_C|SetAngolo%20di%20sterzata (Variables|Default|GetAnimInstance) 0.0)))))

(fn ConstructionScript)