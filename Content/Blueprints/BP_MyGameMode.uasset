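; Game mode Blueprint that keeps an elapsed-time counter while TimerAttivo is true.
; Tick adds a fixed step to Milliseconds, ignoring delta time, and rolls it into Seconds at one, so the count depends on frame rate.
; StartTimer is empty, and a delay-based chain that would roll Seconds into Minutes is disconnected, so Minutes never advances here.
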(event Custom|StartTimer)

(event EventBeginPlay)

(event EventTick
  (params (DeltaSeconds :type Float%20%28single-precision%29))
  (if (Variables|Default|GetTimerAttivo)
    (bind _output_get (Variables|Default|Setmilliseconds (+ (Variables|Default|Getmilliseconds) 0.02)))
    (if (>= _output_get 1.0)
      (Variables|Default|Setseconds (+ (Variables|Default|Getseconds) 1))
      (Variables|Default|Setmilliseconds 0.0))))

(fn ConstructionScript)