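; Motorbike path actor that builds a spline for the selected PathFolder and replays traffic cone changes along that course.
; GeneraProva loads generated path points into the spline, then loads cone data and shifts cones absent at the start to world X/Y zero.
; Tick counts frames, matching cone data to numerically named StaticMeshActors to move, clear or tip them, showing the ConoToccato widget for touched cones.
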(event Custom|AddPointsV2
  (bind _spline (Variables|Default|GetSpline))
  (for _array_element (Variables|Default|GetMotorBikePath)
    (Spline|AddSplinePointatIndex _spline _array_element (Spline|GetNumberOfSplinePoints _spline) "World" true))
  (Utilities|Array|Clear (Variables|Default|GetMotorBikePath)))

(event Custom|processCones
  ;[1 1 1] Porzione di codice che elimina i coni che non sono presenti fin dall'inizio del percorso
  (Class|MyBlueprintFunctionLibrary|GenerateTrafficConeInitialPosition (Utilities|String|EnumtoString (Variables|Default|GetPathFolder)))
  (bind _returnvalue (Class|MyBlueprintFunctionLibrary|ReturnTrafficConeInitialPosition))
  (Variables|Default|SettrafficConesInfo _returnvalue)
  (bind _outactors (Actor|GetAllActorsOfClass "/Script/Engine.StaticMeshActor"))
  (for _array_element _outactors
    (for _index (range 1 76)
      (Development|PrintString (Utilities|GetDisplayName _array_element) false)
      (if (== _index (Math|Conversions|ToInteger(Byte) (Utilities|GetDisplayName _array_element)))
        (switch int (Math|Float|Truncate (.Y (Math|Vector4|BreakVector4 (Utilities|Array|Get(acopy) (Variables|Default|GettrafficConesInfo) _index))))
          (:0
            (Transformation|AddActorWorldOffset _array_element (Math|Vector|MakeVector (* (.x (Transformation|GetActorLocation _array_element)) -1.0) (* (.y (Transformation|GetActorLocation _array_element)) -1.0) 0.0))))))))

(event Custom|AddPoints
  ;[1 1 1] Creazione del percorso
  (Spline|SetSplinePoints (Variables|Default|GetSpline) (Variables|Default|GetMotorBikePath) "World" true)
  (Utilities|Array|Clear (Variables|Default|GetMotorBikePath)))

(event Custom|NumberOfPoints
  (Development|PrintText (Utilities|Text|ToText(Integer) (Spline|GetNumberOfSplinePoints (Variables|Default|GetSpline))) true true "(R=0.000000,G=0.660000,B=1.000000,A=1.000000)" 5.0))

(event Custom|NewMotorBikePath
  ;[1 1 1] Creazione del percorso
  (bind _returnvalue (Class|MyBlueprintFunctionLibrary|GenerateMotorBikePath (Utilities|String|EnumtoString (Variables|Default|GetPathFolder))))
  (for _array_element _returnvalue
    (Development|PrintString _array_element false)))

(event Custom|setMotorBikePath
  ;[1 1 1] Creazione del percorso
  (bind _returnvalue (Class|MyBlueprintFunctionLibrary|ReturnMotorBikePath))
  (Variables|Default|SetMotorBikePath _returnvalue)
  (Class|MyBlueprintFunctionLibrary|CleanMotorBikePath))

(event Custom|Genera%20Prova
  ;[1 1 1] Creazione del percorso
  (CallFunction|NewMotorBikePath)
  (CallFunction|SetMotorBikePath)
  (CallFunction|AddPoints)
  (CallFunction|ProcessCones))

(event EventTick
  (params (DeltaSeconds :type Float%20%28single-precision%29))
  ;[1 1 1] Sezione che gestisce lo spostamento dei coni
  (Variables|Default|Setframe (+ (Variables|Default|Getframe) 1))
  (bind _outactors (Actor|GetAllActorsOfClass "/Script/Engine.StaticMeshActor"))
  (for _array_element _outactors
    (for _index (range 1 76)
      (if (== _index (Math|Conversions|ToInteger(Byte) (Utilities|GetDisplayName _array_element)))
        (if (== (.X (Math|Vector4|BreakVector4 (Utilities|Array|Get(acopy) (Variables|Default|GettrafficConesInfo) _index))) (Variables|Default|Getframe))
          (switch int (Math|Float|Truncate (.Y (Math|Vector4|BreakVector4 (Utilities|Array|Get(acopy) (Variables|Default|GettrafficConesInfo) _index))))
            (:2
              (Transformation|AddActorWorldOffset _array_element (Math|Vector|MakeVector (- (.Z (Math|Vector4|BreakVector4 (Utilities|Array|Get(acopy) (Variables|Default|GettrafficConesInfo) _index))) (.x (Transformation|GetActorLocation _array_element))) (- (.W (Math|Vector4|BreakVector4 (Utilities|Array|Get(acopy) (Variables|Default|GettrafficConesInfo) _index))) (.y (Transformation|GetActorLocation _array_element))) 0.0)))
            (:3
              (Transformation|AddActorWorldOffset _array_element (Math|Vector|MakeVector (* (.x (Transformation|GetActorLocation _array_element)) -1.0) (* (.y (Transformation|GetActorLocation _array_element)) -1.0) 0.0)))
            (:4
              (Transformation|AddActorWorldOffset _array_element (Math|Vector|MakeVector (- (.Z (Math|Vector4|BreakVector4 (Utilities|Array|Get(acopy) (Variables|Default|GettrafficConesInfo) _index))) (.x (Transformation|GetActorLocation _array_element))) (- (.W (Math|Vector4|BreakVector4 (Utilities|Array|Get(acopy) (Variables|Default|GettrafficConesInfo) _index))) (.y (Transformation|GetActorLocation _array_element))) -15.0))
              (Transformation|SetActorRotation _array_element "-90.000000,20.000000,0.000000")
              (bind _returnvalue (UserInterface|CreateWidget "/Game/Blueprints/ConoToccato.ConoToccato_C"))
              (UserInterface|Viewport|AddtoViewport _returnvalue 0))))))))

(fn ConstructionScript)